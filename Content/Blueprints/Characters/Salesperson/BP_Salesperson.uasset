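; Salesperson character whose 2D flipbook sprite changes with the angle it is viewed from, giving a directional-sprite look.
; Every Tick, SetAnimation reads the angle between active camera and flipbook from FlipbookRotator and picks the back, left, right, front-left or front-right flipbook.
; It saves and restores the playback position around each swap so the animation continues seamlessly, and prints a message if the rotator is invalid.
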(event `self.ReceiveTick`
  (params (DeltaSeconds :type "Float (single-precision)"))
  (`parent.ReceiveTick` DeltaSeconds)
  (`self.SetAnimation`))

(fn `SetAnimation`
  (bind _sprite (`self.Sprite`))
  (bind _flipbookrotator (`self.FlipbookRotator`))
  (bind _returnvalue (`FlipbookRotatorComponent.GetDegreesBetweenActiveCameraAndFlipbook` _flipbookrotator))
  (`/Engine/EditorBlueprintResources/StandardMacros.IsValid` _flipbookrotator
    (:`Is Valid`
      (set `self.CurrentAnimationPosition` (`PaperFlipbookComponent.GetPlaybackPosition` (`self.Sprite`)))
      (if (or (> _returnvalue 135.0) (< _returnvalue -135.0))
        (`PaperFlipbookComponent.SetFlipbook` _sprite "/Game/Blueprints/Characters/Salesperson/Flipbooks/FB_Salesperson_Back.FB_Salesperson_Back")
        (elif (and (> _returnvalue -135.0) (< _returnvalue -45.0))
          (`PaperFlipbookComponent.SetFlipbook` _sprite "/Game/Blueprints/Characters/Salesperson/Flipbooks/FB_Salesperson_Left.FB_Salesperson_Left")
          (elif (and (> _returnvalue 45.0) (< _returnvalue 135.0))
            (`PaperFlipbookComponent.SetFlipbook` _sprite "/Game/Blueprints/Characters/Salesperson/Flipbooks/FB_Salesperson_Right.FB_Salesperson_Right")
            (elif (and (> _returnvalue 0.0) (< _returnvalue 45.0))
              (`PaperFlipbookComponent.SetFlipbook` _sprite "/Game/Blueprints/Characters/Salesperson/Flipbooks/FB_Salesperson_FrontRight.FB_Salesperson_FrontRight")
              (else
                (`PaperFlipbookComponent.SetFlipbook` _sprite "/Game/Blueprints/Characters/Salesperson/Flipbooks/FB_Salesperson_FrontLeft.FB_Salesperson_FrontLeft"))))))
      (`PaperFlipbookComponent.SetPlaybackPosition` _sprite (`self.CurrentAnimationPosition`) false))
    (:`Is Not Valid`
      (`KismetSystemLibrary.PrintString` "ROTATOR NOT VALID"))))

(fn `UserConstructionScript`
  (`parent.UserConstructionScript`))