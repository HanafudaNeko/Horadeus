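; Salesperson pawn drawn as a 2D Paper flipbook that shows a different directional sprite depending on the viewing camera's angle.
; Every tick, SetAnimation reads the angle between the active camera and the flipbook from FlipbookRotator.
; It picks a back, left, right, front-right or front-left flipbook from angle ranges.
; The playback position is saved and restored around the swap so the animation continues seamlessly.
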(event `self.ReceiveTick`
  (params (DeltaSeconds :type "Float (single-precision)"))
  (`self.SetAnimation`))

(fn `SetAnimation`
  (locals (CurrentAnimationPosition :type "Float (double-precision)" :default 0.0))
  (bind _paperflipbook (`self.PaperFlipbook`))
  (bind _returnvalue (`FlipbookRotatorComponent.GetDegreesBetweenActiveCameraAndFlipbook` (`self.FlipbookRotator`)))
  (set `local.CurrentAnimationPosition` (`PaperFlipbookComponent.GetPlaybackPosition` (`self.PaperFlipbook`)))
  (if (or (> _returnvalue 135.0) (< _returnvalue -135.0))
    (`PaperFlipbookComponent.SetFlipbook` _paperflipbook "/Game/Characters/Salesperson/Flipbooks/FB_Salesperson_Back.FB_Salesperson_Back")
    (elif (and (> _returnvalue -135.0) (< _returnvalue -45.0))
      (`PaperFlipbookComponent.SetFlipbook` _paperflipbook "/Game/Characters/Salesperson/Flipbooks/FB_Salesperson_Left.FB_Salesperson_Left")
      (elif (and (> _returnvalue 45.0) (< _returnvalue 135.0))
        (`PaperFlipbookComponent.SetFlipbook` _paperflipbook "/Game/Characters/Salesperson/Flipbooks/FB_Salesperson_Right.FB_Salesperson_Right")
        (elif (and (> _returnvalue 0.0) (< _returnvalue 45.0))
          (`PaperFlipbookComponent.SetFlipbook` _paperflipbook "/Game/Characters/Salesperson/Flipbooks/FB_Salesperson_FrontRight.FB_Salesperson_FrontRight")
          (else
            (`PaperFlipbookComponent.SetFlipbook` _paperflipbook "/Game/Characters/Salesperson/Flipbooks/FB_Salesperson_FrontLeft.FB_Salesperson_FrontLeft"))))))
  (`PaperFlipbookComponent.SetPlaybackPosition` _paperflipbook (`local.CurrentAnimationPosition`) false))

(fn `UserConstructionScript`)